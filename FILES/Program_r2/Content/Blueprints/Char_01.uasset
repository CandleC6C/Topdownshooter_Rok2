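; Player character Blueprint that moves along fixed world axes and turns to face the direction of mouse movement.
; Forward and left axis inputs add movement along world X and Y, independent of facing.
; Each tick, mouse delta divided by frame time gives a velocity.
; When its length exceeds a deadzone, the control rotation interpolates toward a yaw derived from that velocity via Atan2, so small movements are ignored.
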(event `InputAxis|Move forward`
  (params (AxisValue :type "Float (single-precision)"))
  (`self.AddMovementInput` (1.0 0.0 0.0) AxisValue))

(event `self.ReceiveTick`
  (params (DeltaSeconds :type "Float (single-precision)"))
  (`self.update player rotation`))

(event `InputAxis|Move Left`
  (params (AxisValue :type "Float (single-precision)"))
  (`self.AddMovementInput` (0.0 1.0 0.0) AxisValue))

(fn `is mouse above deadzone`
  (returns (ReturnValue :type Boolean))
  (return (> (`KismetMathLibrary.VSize2D` (`self.mouse velocity`)) (`self.MouseDeadZone`))))

(fn `mouse velocity`
  (returns (ReturnValue :type "Vector2D Structure"))
  (bind (_deltax _deltay) (`PlayerController.GetInputMouseDelta` (`GameplayStatics.GetPlayerController` 0)))
  (return (/ (`KismetMathLibrary.MakeVector2D` _deltax _deltay) (`GameplayStatics.GetWorldDeltaSeconds`))))

(fn `update player rotation`
  (bind (_returnvalue_x _returnvalue_y) (`KismetMathLibrary.BreakVector2D` (`self.mouse velocity`)))
  (bind _returnvalue (`GameplayStatics.GetPlayerController` 0))
  (if (`self.is mouse above deadzone`)
    (`Controller.SetControlRotation` _returnvalue (`KismetMathLibrary.RInterpTo` (`self.K2_GetActorRotation` _returnvalue) (`KismetMathLibrary.MakeRotator` 0.0 0.0 (`KismetMathLibrary.DegAtan2` _returnvalue_x _returnvalue_y)) (`GameplayStatics.GetWorldDeltaSeconds`) 10.0))))

(fn `UserConstructionScript`)